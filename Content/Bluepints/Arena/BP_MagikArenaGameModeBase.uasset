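; Arena game mode Blueprint that respawns players at random PlayerStart points.
; On BeginPlay it caches every PlayerStart in the level.
; Respawn casts the controller to ArenaPlayerController, destroys any pawn it controls, then spawns the character class from its PlayerInfo at a random cached start.
; The controller then owns and possesses the new pawn.
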(event `self.ReceiveBeginPlay`
  (bind _outactors (`GameplayStatics.GetAllActorsOfClass` "/Script/Engine.PlayerStart"))
  (set `self.SpawnPoints` _outactors))

(event `self.Respawn`
  (params (PlayerController :type "PlayerController Object Reference"))
  (bind _asarena_player_controller (cast `/Game/Bluepints/Arena/ArenaPlayerController` PlayerController))
  (`self.RespawnPlayer` _asarena_player_controller))

(event `RespawnPlayer`
  (params (PlayerController :type "/Game/Bluepints/Arena/ArenaPlayerController Object Reference"))
  (bind _returnvalue (`Controller.K2_GetPawn` PlayerController))
  (bind (_playerinfo_myplayername _playerinfo_myplayercharacter) (break `/Game/Bluepints/AllLevels/PlayerInfo` (`/Game/Bluepints/Arena/ArenaPlayerController.PlayerInfo` PlayerController)))
  (`KismetSystemLibrary.PrintString` "RespawnCalled")
  (`/Engine/EditorBlueprintResources/StandardMacros.IsValid` _returnvalue
    (:`Is Valid`
      (`self.K2_DestroyActor` _returnvalue))
    (:`Is Not Valid`
      _))
  (bind _returnvalue_2 (`self.Get Random Player Start Transform`))
  (bind _returnvalue_3 (`|SpawnActorFromClass` _playerinfo_myplayercharacter _returnvalue_2 "Undefined" "OverrideRootScale" PlayerController null))
  (`Controller.Possess` PlayerController _returnvalue_3))

(fn `Get Random Player Start Transform`
  (returns (ReturnValue :type "Transform Structure (by ref)"))
  (bind _spawnpoints (`self.SpawnPoints`))
  (bind _result (`/Engine/EditorBlueprintResources/StandardMacros.DecrementInt` (`KismetArrayLibrary.Array_Length` _spawnpoints))
    (:`  `
      (return (`self.GetTransform` (`|GetArrayItem` _spawnpoints (`KismetMathLibrary.RandomIntegerInRange` 0 _result)))))))

(fn `UserConstructionScript`)